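; Blueprint function library that returns input prompt icons for keys and buttons on PC, PS, XB, VIdx, HV and OQ devices.
; Each device has its own getter, which picks a Light or Dark search DataTable from the Theme argument.
; The row name comes from the key's long display name after an underscore string replace, and that row's Icon is returned.
; Failed lookups have no separate handling.
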(fn GetPCKeyTexture
  (params (Key :type Key%20Structure :default "A") (Theme :type EInputIconTheme%20Enum :default "NewEnumerator0"))
  (bind _returnvalue (Utilities|GetDataTableRow (Utilities|Select :Index Theme :NewEnumerator0 "/Game/OutbreakZ/Input/InputKeysIcon/DataTables/_SearchTables/PC/DT_PC-Light_SearchTable.DT_PC-Light_SearchTable" :NewEnumerator1 "/Game/OutbreakZ/Input/InputKeysIcon/DataTables/_SearchTables/PC/DT_PC-Dark_SearchTable.DT_PC-Dark_SearchTable") (Utilities|String|StringToName (Utilities|String|Replace (Utilities|String|ToString(Text) (Class|KismetInputLibrary|KeyGetDisplayName Key true)) " " "_")))
    (:then
      _)
    (:RowNotFound
      _))
  (return (Utilities|Struct|BreakFInputIconRow _returnvalue)))

(fn GetPSButtonTexture
  (params (Button :type Key%20Structure :default "A") (Theme :type EInputIconTheme%20Enum :default "NewEnumerator0"))
  (bind _returnvalue (Utilities|GetDataTableRow (Utilities|Select :Index Theme :NewEnumerator0 "/Game/OutbreakZ/Input/InputKeysIcon/DataTables/_SearchTables/PS/DT_PS-Light_SearchTable.DT_PS-Light_SearchTable" :NewEnumerator1 "/Game/OutbreakZ/Input/InputKeysIcon/DataTables/_SearchTables/PS/DT_PS-Dark_SearchTable.DT_PS-Dark_SearchTable") (Utilities|String|StringToName (Utilities|String|Replace (Utilities|String|ToString(Text) (Class|KismetInputLibrary|KeyGetDisplayName Button true)) " " "_")))
    (:then
      _)
    (:RowNotFound
      _))
  (return (Utilities|Struct|BreakFInputIconRow _returnvalue)))

(fn GetXBButtonTexture
  (params (Button :type Key%20Structure :default "A") (Theme :type EInputIconTheme%20Enum :default "NewEnumerator0"))
  (bind _returnvalue (Utilities|GetDataTableRow (Utilities|Select :Index Theme :NewEnumerator0 "/Game/OutbreakZ/Input/InputKeysIcon/DataTables/_SearchTables/XB/DT_XB-Light_SearchTable.DT_XB-Light_SearchTable" :NewEnumerator1 "/Game/OutbreakZ/Input/InputKeysIcon/DataTables/_SearchTables/XB/DT_XB-Dark_SearchTable.DT_XB-Dark_SearchTable") (Utilities|String|StringToName (Utilities|String|Replace (Utilities|String|ToString(Text) (Class|KismetInputLibrary|KeyGetDisplayName Button true)) " " "_")))
    (:then
      _)
    (:RowNotFound
      _))
  (return (Utilities|Struct|BreakFInputIconRow _returnvalue)))

(fn GetVIdxButtonTexture
  (params (Button :type Key%20Structure :default "A") (Theme :type EInputIconTheme%20Enum :default "NewEnumerator0"))
  (bind _returnvalue (Utilities|GetDataTableRow (Utilities|Select :Index Theme :NewEnumerator0 "/Game/OutbreakZ/Input/InputKeysIcon/DataTables/_SearchTables/VIdx/DT_VIdx-Light_SearchTable.DT_VIdx-Light_SearchTable" :NewEnumerator1 "/Game/OutbreakZ/Input/InputKeysIcon/DataTables/_SearchTables/VIdx/DT_VIdx-Dark_SearchTable.DT_VIdx-Dark_SearchTable") (Utilities|String|StringToName (Utilities|String|Replace (Utilities|String|ToString(Text) (Class|KismetInputLibrary|KeyGetDisplayName Button true)) " " "_")))
    (:then
      _)
    (:RowNotFound
      _))
  (return (Utilities|Struct|BreakFInputIconRow _returnvalue)))

(fn GetHVButtonTexture
  (params (Button :type Key%20Structure :default "A") (Theme :type EInputIconTheme%20Enum :default "NewEnumerator0"))
  (bind _returnvalue (Utilities|GetDataTableRow (Utilities|Select :Index Theme :NewEnumerator0 "/Game/OutbreakZ/Input/InputKeysIcon/DataTables/_SearchTables/HV/DT_HV-Light_SearchTable.DT_HV-Light_SearchTable" :NewEnumerator1 "/Game/OutbreakZ/Input/InputKeysIcon/DataTables/_SearchTables/HV/DT_HV-Dark_SearchTable.DT_HV-Dark_SearchTable") (Utilities|String|StringToName (Utilities|String|Replace (Utilities|String|ToString(Text) (Class|KismetInputLibrary|KeyGetDisplayName Button true)) " " "_")))
    (:then
      _)
    (:RowNotFound
      _))
  (return (Utilities|Struct|BreakFInputIconRow _returnvalue)))

(fn GetOQButtonTexture
  (params (Button :type Key%20Structure :default "A") (Theme :type EInputIconTheme%20Enum :default "NewEnumerator0"))
  (bind _returnvalue (Utilities|GetDataTableRow (Utilities|Select :Index Theme :NewEnumerator0 "/Game/OutbreakZ/Input/InputKeysIcon/DataTables/_SearchTables/OQ/DT_OQ-Light_SearchTable.DT_OQ-Light_SearchTable" :NewEnumerator1 "/Game/OutbreakZ/Input/InputKeysIcon/DataTables/_SearchTables/OQ/DT_OQ-Dark_SearchTable.DT_OQ-Dark_SearchTable") (Utilities|String|StringToName (Utilities|String|Replace (Utilities|String|ToString(Text) (Class|KismetInputLibrary|KeyGetDisplayName Button true)) " " "_")))
    (:then
      _)
    (:RowNotFound
      _))
  (return (Utilities|Struct|BreakFInputIconRow _returnvalue)))