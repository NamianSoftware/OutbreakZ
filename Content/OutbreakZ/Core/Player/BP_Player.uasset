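; BP_Player is the OutbreakZ player pawn, adding mobile touch controls for movement and looking.
; Touch and possession events forward to the UTC input and possession manager components.
; On BeginPlay it sets up the movement joystick's screen bounds, widget and priority; the orientation joystick gets no setup here.
; Joystick axis events drive MoveForward/MoveRight with scaled values and LookRight/LookUp, with vertical look inverted.
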(event EventBeginPlay
  (CallFunction|InitializeMobileInput))

(event Collision|EventActorBeginOverlap
  (params (OtherActor :type Actor%20Object%20Reference)))

(event EventTick
  (params (DeltaSeconds :type Float%20%28single-precision%29)))

(event OnXAxisChanged(MovementJoystick)
  (params (Value :type Float%20%28double-precision%29))
  ;[0 0 0] MovementJoystick Inputs
  (Class|SurvivalCharacter|MoveRight (* Value 5e+01)))

(event OnYAxisChanged(MovementJoystick)
  (params (Value :type Float%20%28double-precision%29))
  ;[0 0 0] MovementJoystick Inputs
  (Class|SurvivalCharacter|MoveForward (* Value 5e+01)))

(event OnXAxisChanged(OrientationJoystick)
  (params (Value :type Float%20%28double-precision%29))
  ;[0 0 0] OrientationJoystick
  (Class|SurvivalCharacter|LookRight Value))

(event OnYAxisChanged(OrientationJoystick)
  (params (Value :type Float%20%28double-precision%29))
  ;[0 0 0] OrientationJoystick
  (Class|SurvivalCharacter|LookUp (* Value -1.0)))

(event Custom|InitializeMobileInput
  (bind _movementjoystick (Variables|MobileInput|GetMovementJoystick))
  ;[0 0 0] Initialize
  (Utilities|FlowControl|Sequence
    (:then_0
      ;;[0 0 0] Setup Movement Joystick
      (Default|SetupBounds _movementjoystick true "(X=0.000000,Y=0.500000)" "(X=0.300000,Y=0.500000)" true false)
      (Default|SetupWidget _movementjoystick "/Game/OutbreakZ/Input/Mobile/Widgets/AnimatedWidgets/JoystickWidgetAnimated_v2.JoystickWidgetAnimated_v2_C" true true))
    (:then_1
      ;;[0 0 0] Setup Priority
      (Variables|/Game/OutbreakZ/Input/Mobile/Core/UTCComponent.UTCComponent_C|SetPriority (Variables|MobileInput|GetMovementJoystick) 1))))

(event EventPossessed
  (params (NewController :type Controller%20Object%20Reference))
  ;[0 0 0] Required events to all UTC components
  (Utilities|UTCPawnPossesionManager NewController (stale EventUnpossessed OldController)))

(event EventUnpossessed
  (params (OldController :type Controller%20Object%20Reference))
  ;[0 0 0] Required events to all UTC components
  (Utilities|UTCPawnPossesionManager (stale EventPossessed NewController) OldController) ; enters at Unpossesed
)

(event Input|TouchEvents|InputTouch
  (params (Location :type Vector) (FingerIndex :type ETouchIndex%20Enum))
  ;[0 0 0] Required events to all UTC components
  (:Pressed
    (Utilities|UTCTouchInputManager Location FingerIndex :!label _label))
  (:Released
    (goto _label Released))
  (:Moved
    (goto _label Moved)))

(fn ConstructionScript)