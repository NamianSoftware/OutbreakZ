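; BP_LadderMaster is a ladder prop that builds itself procedurally from a height setting in the construction script.
; It scales both side poles to the height, then loops upward by a fixed gap, adding instanced rungs and optional screw pairs at set intervals.
; It also moves the exit area and ExitBot components to the computed top.
; The event graph holds no logic.
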(event EventBeginPlay)

(event Collision|EventActorBeginOverlap
  (params (OtherActor :type Actor%20Object%20Reference)))

(event EventTick
  (params (DeltaSeconds :type Float%20%28single-precision%29)))

(fn ConstructionScript
  (bind _rightladderpole (Variables|Default|GetRightLadderPole))
  (bind _leftladderpole (Variables|Default|GetLeftLadderPole))
  (bind _screwsinstance (Variables|Default|GetScrewsInstance))
  (bind _ladderheight (Variables|LadderSettings|GetLadderHeight))
  (bind _ladderheightmultiplier (Variables|Private|GetLadderHeightMultiplier))
  (bind _returnvalue (Transformation|GetWorldScale _rightladderpole))
  (bind _returnvalue_2 (Transformation|GetWorldScale _leftladderpole))
  (bind _returnvalue_3 (* _ladderheight _ladderheightmultiplier))
  (Transformation|SetRelativeScale3D _rightladderpole (Math|Vector|MakeVector (.x _returnvalue) (.y _returnvalue) (Variables|LadderSettings|GetLadderHeight)))
  (Transformation|SetRelativeScale3D _leftladderpole (Math|Vector|MakeVector (.x _returnvalue_2) (.y _returnvalue_2) (Variables|LadderSettings|GetLadderHeight)))
  (Variables|Private|SetCompareHeight (Variables|LadderSettings|GetLadderBarsOffet))
  (while (< (Variables|Private|GetCompareHeight) (* (Variables|LadderSettings|GetLadderHeight) (Variables|Private|GetLadderHeightMultiplier)))
    ;[0 0 0] Cycle
    (Math|Integer|IncrementInt (Variables|Private|GetLoopIndex)
      (:%20%20
        (Utilities|FlowControl|Sequence
          (:then_0
            ;;[0 0 0] Bars
            (Components|InstancedStaticMesh|AddInstance (Variables|Default|GetBarsInstance) (Math|Transform|MakeTransform (Math|Vector|MakeVector 0.0 0.0 (Variables|Private|GetCompareHeight)) "0, 0, 0" "1.000000,1.000000,1.000000") false))
          (:then_1
            (if (Variables|LadderSettings|GetHasScrews?)
              (if (== (Math|Integer|%(Integer) (Variables|Private|GetLoopIndex) (Variables|LadderSettings|GetScrewsInterval)) 0)
                (Components|InstancedStaticMesh|AddInstance _screwsinstance (Math|Transform|MakeTransform (Math|Vector|MakeVector 25.0 -14.0 (- (Variables|Private|GetCompareHeight) (Variables|LadderSettings|GetLadderGap))) "0.000000,-90.000000,0.000000" "1.000000,1.000000,1.000000") false)
                (Components|InstancedStaticMesh|AddInstance _screwsinstance (Math|Transform|MakeTransform (Math|Vector|MakeVector -25.0 -14.0 (- (Variables|Private|GetCompareHeight) (Variables|LadderSettings|GetLadderGap))) "0.000000,-90.000000,0.000000" "1.000000,1.000000,1.000000") false))))
          (:then_2
            (Variables|Private|SetCompareHeight (+ (Variables|Private|GetCompareHeight) (Variables|LadderSettings|GetLadderGap))))))))
  (Transformation|SetRelativeLocation (Variables|Default|GetLadderExitArea) (Math|Vector|MakeVector 0.0 0.0 _returnvalue_3) false false)
  (Transformation|SetRelativeLocation (Variables|Default|GetExitBot) (Math|Vector|MakeVector 0.0 25.0 (+ (Variables|Default|GetExitBoxOffset) _returnvalue_3)) false false))